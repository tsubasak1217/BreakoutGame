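; BP_Ball is the bouncing ball of a paddle game, counted in BP_GameManager's FieldBallCount from spawn until destroyed.
; Tick moves it along Direction at Speed with a swept move, and hits mirror Direction about the surface normal and play a sound.
; Paddle top hits use the paddle's GetTopNormal and ClampDirection, whose angle-limit math appears unused.
; Overlapping a MissArea component decrements the count and destroys the ball.
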(event OnComponentBeginOverlap(ball)
  (params (OverlappedComponent :type Primitive%20Component%20Object%20Reference) (OtherActor :type Actor%20Object%20Reference) (OtherComp :type Primitive%20Component%20Object%20Reference) (OtherBodyIndex :type Integer) (bFromSweep :type Boolean) (SweepResult :type Hit%20Result%20Structure%20%28by%20ref%29))
  ;[0.15 0.15 0.15 0.5] 下に落ちたら消滅処理
  (if (Components|ComponentHasTag OtherComp "MissArea")
    (bind _returnvalue (Actor|GetActorOfClass "/Game/Actors/BP_GameManager.BP_GameManager_C"))
    (Math|Integer|DecrementInt (Variables|/Game/Actors/BP_GameManager.BP_GameManager_C|GetFieldBallCount _returnvalue)
      (:%20%20
        (Actor|DestroyActor)))))

(event EventBeginPlay
  ;[0.15 0.15 0.15 0.5] 生成時にフィールド上の弾の数を加算
  (bind _returnvalue (Actor|GetActorOfClass "/Game/Actors/BP_GameManager.BP_GameManager_C"))
  (Math|Integer|IncrementInt (Variables|/Game/Actors/BP_GameManager.BP_GameManager_C|GetFieldBallCount _returnvalue)))

(event Collision|EventActorBeginOverlap
  (params (OtherActor :type Actor%20Object%20Reference)))

(event EventTick
  (params (DeltaSeconds :type Float%20%28single-precision%29))
  (Transformation|SetActorLocation (+ (Transformation|GetActorLocation) (* (* (Variables|Default|Getspeed) (Math|Vector|Normalize (Variables|Default|Getdirection))) (Utilities|Time|GetWorldDeltaSeconds))) true false))

(event Collision|EventHit
  (params (MyComp :type Primitive%20Component%20Object%20Reference) (Other :type Actor%20Object%20Reference) (OtherComp :type Primitive%20Component%20Object%20Reference) (bSelfMoved :type Boolean) (HitLocation :type Vector :default "0, 0, 0") (HitNormal :type Vector :default "0, 0, 0") (NormalImpulse :type Vector :default "0, 0, 0") (Hit :type Hit%20Result%20Structure%20%28by%20ref%29))
  ;[0.15 0.15 0.15 0.5] 当たったら反射
  (if (Components|ComponentHasTag OtherComp "Player")
    (bind _asbp_paddle (Utilities|Casting|CastToBP_Paddle Other)
      (:then
        (bind (_ishittopsurface _outnormal) (Default|GetTopNormal _asbp_paddle HitLocation HitNormal))
        (if _ishittopsurface
          (Variables|Default|Setdirection (Utilities|ClampDirection (Math|Vector|MirrorVectorbyNormal (Variables|Default|Getdirection) _outnormal)))
          (else
            (Variables|Default|Setdirection (Math|Vector|MirrorVectorbyNormal (Variables|Default|Getdirection) HitNormal) :!label _label))))
      (:CastFailed
        (goto _label)))
    (else
      (goto _label)))
  (Audio|PlaySound2D "/Game/Audios/hit1.hit1" 1.0 1.0 0.0 0 0))

(fn ConstructionScript)