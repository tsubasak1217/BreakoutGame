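; Player paddle actor that slides sideways with swept movement on Enhanced Input and forwards the action input to BP_GameManager.
; GetTopNormal tilts straight-up hit normals in proportion to the hit's Y offset from center, up to MaxTintNormalDeg at the edges, and flags top-surface hits.
; Tick samples that function across the top surface and draws debug arrows to visualize the resulting normals.
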(event Input|EnhancedActionEvents|EnhancedInputActionIA_Move
  (params (ActionValue :type Float%20%28double-precision%29) (ElapsedSeconds :type Float%20%28double-precision%29) (TriggeredSeconds :type Float%20%28double-precision%29) (InputAction :type Input%20Action%20Object%20Reference :default "/Game/Input/IA_Move.IA_Move"))
  (Transformation|SetActorLocation (+ (* (* (Class|KismetMathLibrary|VectorRight) ActionValue) (* (Variables|Default|Getspeed) (Utilities|Time|GetWorldDeltaSeconds))) (Transformation|GetActorLocation)) true false))

(event Input|EnhancedActionEvents|EnhancedInputActionIA_Action
  (params (ActionValue :type Boolean) (ElapsedSeconds :type Float%20%28double-precision%29) (TriggeredSeconds :type Float%20%28double-precision%29) (InputAction :type Input%20Action%20Object%20Reference :default "/Game/Input/IA_Action.IA_Action"))
  (:Started
    (Default|Action (Variables|Default|GetGameManager))))

(event EventBeginPlay
  (Input|AddMappingContext (PlayerController|LocalPlayerSubsystems|GetEnhancedInputLocalPlayerSubsystem (Game|GetPlayerController 0)) "/Game/Input/IMC_InGame.IMC_InGame" 0 "(bIgnoreAllPressedKeysUntilRelease=True,bForceImmediately=False,bNotifyUserSettings=False)")
  (bind _returnvalue (Actor|GetActorOfClass "/Game/Actors/BP_GameManager.BP_GameManager_C"))
  (Variables|Default|SetGameManager _returnvalue))

(event Collision|EventActorBeginOverlap
  (params (OtherActor :type Actor%20Object%20Reference)))

(event EventTick
  (params (DeltaSeconds :type Float%20%28single-precision%29))
  (CallFunction|DrawDbgNormals))

(fn ConstructionScript)

(fn GetTopNormal
  (params (HitLocation :type Vector) (HitNormal :type Vector))
  (bind (_origin _boxextent) (Collision|GetActorBounds false false))
  (if (Utilities|Operators|NotEqual(!=) HitNormal (Math|Vector|VectorUp) 0.0)
    (return false HitNormal)
    (else
      (return true (Math|Vector|RotateVector HitNormal (Math|Rotator|MakeRotator (* (/ (- (.Y (Math|Vector|BreakVector HitLocation)) (.y _origin)) (.y _boxextent)) (Variables|Default|GetMaxTintNormalDeg)) 0.0 0.0))))))

(fn DrawDebugArrow
  (params (Origin :type Vector) (Direction :type Vector))
  (LocalVariables|SetL_shapedDirection (* (Math|Vector|Normalize Direction) (LocalVariables|GetL_Length)))
  (Rendering|Debug|DrawDebugArrow Origin (+ Origin (LocalVariables|GetL_shapedDirection)) 1e+02 "(R=0.000000,G=0.084802,B=1.000000,A=1.000000)" 0.0 1e+01))

(fn DrawDbgNormals
  (bind (_origin _boxextent) (Collision|GetActorBounds false false))
  (for _index (range (* (LocalVariables|GetL_DrawCountHalf) -1) (LocalVariables|GetL_DrawCountHalf))
    (bind _outnormal (CallFunction|GetTopNormal (+ (Math|Vector|MakeVector 0.0 (* (/ (.y _boxextent) (LocalVariables|GetL_DrawCountHalf)) _index) (.z _boxextent)) _origin) (Math|Vector|VectorUp)))
    (CallFunction|DrawDebugArrow (+ (Math|Vector|MakeVector 0.0 (* (/ (.y _boxextent) (LocalVariables|GetL_DrawCountHalf)) _index) (.z _boxextent)) _origin) _outnormal)))