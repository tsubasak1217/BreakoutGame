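; BP_Block is a destructible block with hit points that registers itself in the BP_GameManager block count on BeginPlay.
; Each Hit decrements HP, and ReloadHP updates the text label and tints a construction-time dynamic material from ColorTable, indexed by clamped HP.
; At zero HP it decrements the manager's count, destroys itself and randomly spawns an AddBallItem at its location based on ItemSpawnRate.
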(event EventBeginPlay
  (bind _returnvalue (Actor|GetActorOfClass "/Game/Actors/BP_GameManager.BP_GameManager_C"))
  (Default|IncrementBlockCount _returnvalue)
  (CallFunction|ReloadHP))

(event Collision|EventActorBeginOverlap
  (params (OtherActor :type Actor%20Object%20Reference)))

(event EventTick
  (params (DeltaSeconds :type Float%20%28single-precision%29)))

(event Collision|EventHit
  (params (MyComp :type Primitive%20Component%20Object%20Reference) (Other :type Actor%20Object%20Reference) (OtherComp :type Primitive%20Component%20Object%20Reference) (bSelfMoved :type Boolean) (HitLocation :type Vector :default "0, 0, 0") (HitNormal :type Vector :default "0, 0, 0") (NormalImpulse :type Vector :default "0, 0, 0") (Hit :type Hit%20Result%20Structure%20%28by%20ref%29))
  (bind _result (Math|Integer|DecrementInt (Variables|Default|Gethp))
    (:%20%20
      (CallFunction|ReloadHP)
      (if (<= _result 0)
        (bind _returnvalue (Actor|GetActorOfClass "/Game/Actors/BP_GameManager.BP_GameManager_C"))
        (Default|DecrementBlockCount _returnvalue)
        (Actor|DestroyActor)
        (if (<= (Math|Random|RandomFloatinRange 0.0 1.0) (Variables|Default|GetItemSpawnRate))
          (Game|SpawnActorfromClass "/Game/Actors/AddBallItem.AddBallItem_C" (Math|Transform|MakeTransform (Transformation|GetActorLocation) "0, 0, 0" "1.000000,1.000000,1.000000") "Undefined" "MultiplyWithRoot" 0 0))))))

(fn ConstructionScript
  (bind _returnvalue (Rendering|Material|CreateDynamicMaterialInstance (Variables|Default|GetCube) 0 0 "None" :!class /Script/Engine.PrimitiveComponent))
  (Variables|Default|SetMaterialInstance _returnvalue))

(fn ReloadHP
  (bind _hp (Variables|Default|Gethp))
  (Rendering|Components|TextRender|SetText (Variables|Default|GetTextRender) (Utilities|Text|ToText(Integer) _hp))
  (Rendering|Material|SetVectorParameterValue (Variables|Default|GetMaterialInstance) "BaseColor" (Math|Conversions|ToLinearColor(Color) (Utilities|Array|Get(acopy) (Variables|Default|GetColorTable) (Math|Integer|Clamp(Integer) (- _hp 1) 0 (Utilities|Array|LastIndex (Variables|Default|GetColorTable))))) :!class /Script/Engine.MaterialInstanceDynamic))