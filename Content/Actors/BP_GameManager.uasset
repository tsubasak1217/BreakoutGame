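; Game manager actor for a Breakout level, tracking block count, balls in play and balls left.
; BeginPlay restores the ball count from the game instance; Tick shows a clear widget when blocks run out, or game over when no balls remain.
; Action is state-dependent: it spawns a ball, reloads the level after game over, or saves balls plus one and opens the next level after a clear.
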(event EventBeginPlay
  (bind _asbreakout_game_instance (Utilities|Casting|CastToBreakoutGame_Instance (Game|GetGameInstance)))
  (bind _isballcountvaild (Default|CheckIsBallCountVaild _asbreakout_game_instance))
  (if _isballcountvaild
    (Variables|Default|SetBallLeftCount (Variables|/Game/Actors/BreakoutGame_Instance.BreakoutGame_Instance_C|GetleftBallCount _asbreakout_game_instance))))

(event Collision|EventActorBeginOverlap
  (params (OtherActor :type Actor%20Object%20Reference)))

(event EventTick
  (params (DeltaSeconds :type Float%20%28single-precision%29))
  (if (not (or (Variables|Default|GetIsClear) (Variables|Default|GetIsGameOver)))
    ;[0.15 0.15 0.15 0.5] クリア判定
    (bind _returnvalue (CallFunction|ClearCheck))
    (if _returnvalue
      (Variables|Default|SetIsClear true)
      (CallFunction|ViewClearWidget)
      (else
        ;[0.15 0.15 0.15 0.5] ゲームオーバー判定
        (if (and (<= (Variables|Default|GetBallLeftCount) 0) (== (Variables|Default|GetFieldBallCount) 0))
          (Variables|Default|SetIsGameOver true)
          (CallFunction|ViewGameOverWidget))))))

(fn ConstructionScript)

(fn IncrementBlockCount
  (Math|Integer|IncrementInt (Variables|Default|GetblockCount)))

(fn DecrementBlockCount
  (Math|Integer|DecrementInt (Variables|Default|GetblockCount)))

(fn ClearCheck
  (return (<= (Variables|Default|GetblockCount) 0)))

(fn ViewClearWidget
  (bind _returnvalue (UserInterface|CreateWidget "/Game/Actors/ClearWidget.ClearWidget_C"))
  (UserInterface|Viewport|AddtoViewport _returnvalue 0))

(fn ViewGameOverWidget
  (bind _returnvalue (UserInterface|CreateWidget "/Game/Actors/GameOverWidget.GameOverWidget_C"))
  (UserInterface|Viewport|AddtoViewport _returnvalue 0))

(fn SpawnBall
  (if (== (Variables|Default|GetFieldBallCount) 0)
    (Game|SpawnActorfromClass "/Game/Actors/BP_Ball.BP_Ball_C" (Class|GeometryScriptLibraryTransformFunctions|MakeTransformfromAxes (Transformation|GetActorLocation (Variables|Default|GetRespawnLocationActor)) "0, 0, 0" "0, 0, 0" true) "Undefined" "MultiplyWithRoot" 0 0)
    (Variables|Default|SetFieldBallCount (Math|Conversions|ToInteger(Boolean) (Class|KismetSystemLibrary|MakeLiteralBool true)))
    (Math|Integer|DecrementInt (Variables|Default|GetBallLeftCount))))

(fn Action
  (if (Variables|Default|GetIsGameOver)
    (CallFunction|ResetLevel)
    (elif (Variables|Default|GetIsClear)
      (CallFunction|OpenNextLevel)
      (else
        (CallFunction|SpawnBall)))))

(fn ResetLevel
  (bind _returnvalue (Game|GetCurrentLevelName true))
  (Game|OpenLevel(byName) (Utilities|String|StringToName _returnvalue)))

(fn OpenNextLevel
  (bind _asbreakout_game_instance (Utilities|Casting|CastToBreakoutGame_Instance (Game|GetGameInstance)))
  (Variables|/Game/Actors/BreakoutGame_Instance.BreakoutGame_Instance_C|SetleftBallCount _asbreakout_game_instance (+ (Variables|Default|GetBallLeftCount) 1))
  (Game|OpenLevel(byName) (Variables|Default|GetNextLevelName)))

(fn GenerateBall
  (Game|SpawnActorfromClass "/Game/Actors/BP_Ball.BP_Ball_C" (Class|GeometryScriptLibraryTransformFunctions|MakeTransformfromAxes (Transformation|GetActorLocation (Variables|Default|GetRespawnLocationActor)) "0, 0, 0" "0, 0, 0" true) "Undefined" "MultiplyWithRoot" 0 0))